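; Interactive console button actor that takes one of four forms chosen by Type: cylinder, add, subtract or pull lever.
; BeginPlay shows the matching shape and caches its travel limits.
; Tick drives two sub-graphs that animate the shape by hand within those limits, sliding buttons along Z and rolling the lever.
; The button press branch reports ButtonName to Console.ManageButtons and clears IsPressed for Add and Subs; the lever's Console call is unconnected.
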(event EventBeginPlay
  (bind _cylinder (Variables|Default|GetCylinder))
  (bind _returnvalue (Transformation|GetWorldLocation _cylinder))
  (switch int (Variables|Default|Gettype)
    (:0
      (bind _output_get (Variables|Default|SetShape (Variables|Default|GetCylinder)))
      (Variables|Default|SetbuttonLength 2.5)
      (Rendering|SetVisibility _output_get true true))
    (:1
      (bind _output_get_2 (Variables|Default|SetShape (Variables|Default|GetAdd)))
      (Variables|Default|SetbuttonLength 2.5)
      (Rendering|SetVisibility _output_get_2 true true))
    (:2
      (bind _output_get_3 (Variables|Default|SetShape (Variables|Default|GetSubs)))
      (Variables|Default|SetbuttonLength 2.5)
      (Rendering|SetVisibility _output_get_3 true true))
    (:3
      (bind _output_get_4 (Variables|Default|SetShape (Variables|Default|GetPull)))
      (Rendering|SetVisibility _output_get_4 true true)
      (bind _output_get_5 (Variables|Default|SetinitialRot (.roll (Variables|/Script/Engine.SceneComponent|GetRelativeRotation (Variables|Default|GetPullRotator)))))
      (Variables|Default|SetmaxRot (+ _output_get_5 -5e+01))
      (Variables|Default|SetbuttonSpeed -2e+02)))
  (Variables|Default|SetinitialZ (.z _returnvalue))
  (Variables|Default|SetmaxVal (- (.z _returnvalue) (Variables|Default|GetbuttonLength))))

(event Collision|EventActorBeginOverlap
  (params (OtherActor :type Actor%20Object%20Reference)))

(event EventTick
  (params (DeltaSeconds :type Float%20%28single-precision%29))
  (if (and (== (Variables|Default|Gettype) 3) (Variables|Default|GetisPressed))
    (Utilities|PullTypesManagment DeltaSeconds :!label _label
      (:next
        _)
      (:then
        _))
    (if (Variables|Default|GetisPressed)
      (if (not (== (Variables|Default|Gettype) 3))
        (goto _label_2 execute2))
      (elif (not (== (Variables|Default|Gettype) 3))
        (Utilities|ButtonTypesManagment DeltaSeconds DeltaSeconds :!label _label_2)))
    (else
      (goto _label release))))

(fn ConstructionScript)