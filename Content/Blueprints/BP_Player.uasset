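; First-person player for a game that opens on a menu with music and video, then starts on any key with a HUD and alarm.
; A timed blinking intro with a post-process effect hands over to a per-frame camera trace that highlights BP_Button targets on the crosshair.
; Left click presses the targeted button, otherwise swings the Kane weapon through a Tick-driven rotation state.
; Box and KaneCollider overlaps destroy BP_Enemy actors with splash particles.
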(event OnComponentBeginOverlap(Box)
  (params (OverlappedComponent :type Primitive%20Component%20Object%20Reference) (OtherActor :type Actor%20Object%20Reference) (OtherComp :type Primitive%20Component%20Object%20Reference) (OtherBodyIndex :type Integer) (bFromSweep :type Boolean) (SweepResult :type Hit%20Result%20Structure%20%28by%20ref%29))
  (bind _asbp_enemy (Utilities|Casting|CastToBP_Enemy OtherActor))
  (Effects|SpawnEmitteratLocation "/Game/Particles/PT_Enemy_Splash.PT_Enemy_Splash" (Transformation|GetActorLocation _asbp_enemy))
  (Actor|DestroyActor _asbp_enemy))

(event OnComponentBeginOverlap(kaneCollider)
  (params (OverlappedComponent :type Primitive%20Component%20Object%20Reference) (OtherActor :type Actor%20Object%20Reference) (OtherComp :type Primitive%20Component%20Object%20Reference) (OtherBodyIndex :type Integer) (bFromSweep :type Boolean) (SweepResult :type Hit%20Result%20Structure%20%28by%20ref%29))
  (bind _asbp_enemy (Utilities|Casting|CastToBP_Enemy OtherActor))
  (Effects|SpawnEmitteratLocation "/Game/Particles/PT_Enemy_Splash.PT_Enemy_Splash" (Transformation|GetActorLocation _asbp_enemy))
  (Actor|DestroyActor _asbp_enemy))

(event EventBeginPlay
  (bind _mediaplayer (Variables|Default|GetMediaPlayer))
  (Audio|Components|Audio|Play (Variables|Default|GetmenuMusic) 0.0)
  (Class|MediaPlayer|OpenPlaylistIndex _mediaplayer "/Game/Videos/PlayList.PlayList")
  (Media|MediaPlayer|Play _mediaplayer :!class /Script/MediaAssets.MediaPlayer))

(event Collision|EventActorBeginOverlap
  (params (OtherActor :type Actor%20Object%20Reference)))

(event EventTick
  (params (DeltaSeconds :type Float%20%28single-precision%29))
  (if (Variables|Default|GetdoneBlinking)
    (CallFunction|CameraRay)
    (else
      (CallFunction|BlinkIntro DeltaSeconds DeltaSeconds)))
  (if (> (Variables|Default|GetkaneStatus) 0)
    (switch int (Variables|Default|GetkaneStatus)
      (:1
        (if (> (.pitch (Variables|/Script/Engine.SceneComponent|GetRelativeRotation (Variables|Default|GetKaneRotator))) -6e+01)
          (Transformation|AddLocalRotation (Variables|Default|GetKaneRotator) (Math|Rotator|MakeRotator 0.0 (* (Utilities|Time|GetWorldDeltaSeconds) -4e+02) 0.0) false false)
          (else
            (Variables|Default|SetkaneStatus 2)
            (Audio|Components|Audio|Play (Variables|Default|GetsaberSwing) 0.0))))
      (:2
        (if (< (.pitch (Variables|/Script/Engine.SceneComponent|GetRelativeRotation (Variables|Default|GetKaneRotator))) 0.0)
          (Transformation|AddLocalRotation (Variables|Default|GetKaneRotator) (Math|Rotator|MakeRotator 0.0 (* (Utilities|Time|GetWorldDeltaSeconds) 2e+02) 0.0) false false)
          (else
            (Variables|Default|SetkaneStatus 0)))))))

(event Input|AxisEvents|InputAxisMoveForward
  (params (AxisValue :type Float%20%28single-precision%29))
  (if (Variables|Default|GetisPlaying)
    (Pawn|Input|AddMovementInput (Transformation|GetActorForwardVector) (* (Variables|Default|GetMovementSpeed) AxisValue (stale EventTick DeltaSeconds)) false)))

(event Input|AxisEvents|InputAxisMoveRight
  (params (AxisValue :type Float%20%28single-precision%29))
  (Pawn|Input|AddMovementInput (Transformation|GetActorRightVector) (* (Variables|Default|GetMovementSpeed) AxisValue (stale EventTick DeltaSeconds)) false))

(event Input|AxisEvents|InputAxisLookHorizontal
  (params (AxisValue :type Float%20%28single-precision%29))
  (if (Variables|Default|GetisPlaying)
    (Pawn|Input|AddControllerYawInput (* AxisValue (Variables|Default|GetLookSpeed)))))

(event Input|AxisEvents|InputAxisLookVertical
  (params (AxisValue :type Float%20%28single-precision%29))
  (if (Variables|Default|GetisPlaying)
    (Pawn|Input|AddControllerPitchInput (* AxisValue (Variables|Default|GetLookSpeed)))))

(event Input|MouseEvents|LeftMouseButton
  (params (Key :type Key%20Structure))
  (bind _lastbutton (Variables|Default|GetLastButton))
  (:Pressed
    (if (Variables|Default|GetisPlaying)
      (if (Variables|Default|GetcanPressButton)
        (Variables|/Game/Blueprints/BP_Button.BP_Button_C|SetisPressed _lastbutton true)
        (Development|PrintString (Variables|/Game/Blueprints/BP_Button.BP_Button_C|GetbuttonName _lastbutton))
        (elif (== (Variables|Default|GetkaneStatus) 0)
          (Variables|Default|SetkaneStatus 1)
          (Audio|Components|Audio|Play (Variables|Default|GetsaberSwing) 0.0)))))
  (:Released
    (if (Variables|Default|GetisPlaying)
      (if (Utilities|IsValid _lastbutton)
        (Variables|/Game/Blueprints/BP_Button.BP_Button_C|SetisPressed _lastbutton false)))))

(event Input|KeyboardEvents|AnyKey
  (params (Key :type Key%20Structure))
  (:Pressed
    (if (not (Variables|Default|GetisPlaying))
      (Variables|Default|SetisPlaying true)
      (bind _returnvalue (UserInterface|CreateWidget "/Game/Blueprints/WBP_Hud.WBP_Hud_C"))
      (bind _output_get (Variables|Default|SetHUD _returnvalue))
      (UserInterface|Viewport|AddtoViewport _output_get 0)
      (Variables|Default|SetCrossHair (Variables|/Game/Blueprints/WBP_Hud.WBP_Hud_C|GetCross (Variables|Default|GetHUD)))
      (Variables|/Script/Engine.CharacterMovementComponent|SetMaxWalkSpeed (Variables|Character|GetCharacterMovement) 1e+03)
      (Rendering|SetVisibility (Variables|Default|GetPlane) false true)
      (bind _structout (Utilities|Struct|SetmembersinPostProcessSettings (Variables|/Script/Engine.CameraComponent|GetPostProcessSettings (Variables|Default|GetCamera)) "BM_SOG" 6e+02))
      (Variables|/Script/Engine.CameraComponent|SetPostProcessSettings (Variables|Default|GetCamera) _structout)
      (Audio|Components|Audio|Stop (Variables|Default|GetmenuMusic))
      (Audio|Components|Audio|Play (Variables|Default|GetalarmSound) 0.0))))

(fn ConstructionScript)

(fn BlinkEyes
  (bind _hud (Variables|Default|GetHUD))
  (bind _black (Variables|/Game/Blueprints/WBP_Hud.WBP_Hud_C|GetBlack _hud))
  (if (<= (Variables|Default|GetblinkTimer) 0.0)
    (if (Variables|Default|Getblink)
      (Widget|SetVisibility _black (LocalVariables|GetHidden))
      (else
        (Widget|SetVisibility _black (LocalVariables|GetVisible))))
    (Variables|Default|SetblinkTimer 0.5)
    (Variables|Default|Setblink (not (Variables|Default|Getblink)))))

(fn BlinkIntro
  (params (A :type Float%20%28single-precision%29) (B :type Float%20%28single-precision%29))
  (if (and (Variables|Default|GetisPlaying) (>= (Variables|Default|GetfocalDistance) 0.0))
    (bind _output_get (Variables|Default|SetfocalDistance (- (Variables|Default|GetfocalDistance) (* A 2e+06))))
    (if (<= _output_get 0.0)
      (bind _structout (Utilities|Struct|SetmembersinPostProcessSettings (Variables|/Script/Engine.CameraComponent|GetPostProcessSettings (Variables|Default|GetCamera)) "BM_SOG" 0.0))
      (Variables|/Script/Engine.CameraComponent|SetPostProcessSettings (Variables|Default|GetCamera) _structout)
      (Variables|Default|SetdoneBlinking true)
      (Widget|SetVisibility (Variables|/Game/Blueprints/WBP_Hud.WBP_Hud_C|GetBlack (Variables|Default|GetHUD)) "Hidden")
      (else
        (CallFunction|BlinkEyes)
        (Variables|Default|SetblinkTimer (- (Variables|Default|GetblinkTimer) B))))))

(fn CameraRay
  (bind _crosshair (Variables|Default|GetCrossHair))
  (bind _camera (Variables|Default|GetCamera))
  (bind _returnvalue (Transformation|GetWorldLocation _camera))
  (if (Variables|Default|GetisPlaying)
    (bind _outhit (Collision|LineTraceByChannel _returnvalue (+ _returnvalue (* (Math|Vector|GetForwardVector _camera) 1e+04)) "TraceTypeQuery1" false 0 "None"))
    (if true
      (bind _asbp_button (Utilities|Casting|CastToBP_Button (.HitActor (Collision|BreakHitResult _outhit)))
        (:then
          (Appearance|SetColorandOpacity _crosshair "(R=0.019052,G=1.000000,B=0.000000,A=1.000000)" :!class /Script/UMG.Image)
          (Variables|Default|SetLastButton _asbp_button)
          (Variables|Default|SetcanPressButton true))
        (:CastFailed
          (Appearance|SetColorandOpacity _crosshair "(R=1.000000,G=1.000000,B=1.000000,A=1.000000)" :!class /Script/UMG.Image)
          (Variables|Default|SetcanPressButton false))))))