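; Reactor console actor simulating core temperature and four vent valve pressures while the player is playing.
; On BeginPlay it spawns linked BP_Buttons for venting valves and moving refrigeration units to or from GameControl's shared pool.
; Each tick, temperature and pressures feed each other, with fires and refrigeration also affecting heat; valves hitting maximum die and turn emergency material.
; Threshold crossings queue latched temperature and pressure warning sounds in GameControl.
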(event EventBeginPlay
  (bind _asbp_player (Utilities|Casting|CastToBP_Player (Game|Player|GetPlayerPawn 0)))
  (Variables|Default|Setplayer _asbp_player)
  (Rendering|Components|TextRender|SetText (Variables|Default|GetReactorNumber) (Utilities|Text|ToText(String) (Variables|Default|GetconsoleName)))
  (bind _returnvalue (Game|SpawnActorfromClass "/Game/Blueprints/BP_Button.BP_Button_C" (Math|Transform|MakeTransform (Transformation|GetWorldLocation (Variables|Default|GetAddButton)) "0, 0, 0" "0.200000,0.200000,0.200000") "Undefined" 0 "AddButton" 1 0))
  (bind _output_get (Variables|Default|SetAddButtonRef _returnvalue))
  (Variables|/Game/Blueprints/BP_Button.BP_Button_C|Setconsole _output_get self)
  (bind _returnvalue_2 (Game|SpawnActorfromClass "/Game/Blueprints/BP_Button.BP_Button_C" (Math|Transform|MakeTransform (Transformation|GetWorldLocation (Variables|Default|GetSubsButton)) "0, 0, 0" "0.200000,0.200000,0.200000") "Undefined" 0 "SubsButton" 2 0))
  (bind _output_get_2 (Variables|Default|SetSubsButtonRef _returnvalue_2))
  (Variables|/Game/Blueprints/BP_Button.BP_Button_C|Setconsole _output_get_2 self)
  (bind _returnvalue_3 (Game|SpawnActorfromClass "/Game/Blueprints/BP_Button.BP_Button_C" (Math|Transform|MakeTransform (Transformation|GetWorldLocation (Variables|Default|GetVentButton1)) "0, 0, 0" "0.200000,0.200000,0.200000") "Undefined" 0 "" 0 0))
  (bind _output_get_3 (Variables|Default|SetButton1 _returnvalue_3))
  (Variables|/Game/Blueprints/BP_Button.BP_Button_C|Setconsole _output_get_3 self)
  (bind _returnvalue_4 (Game|SpawnActorfromClass "/Game/Blueprints/BP_Button.BP_Button_C" (Math|Transform|MakeTransform (Transformation|GetWorldLocation (Variables|Default|GetVentButton2)) "0, 0, 0" "0.200000,0.200000,0.200000") "Undefined" 0 "" 0 0))
  (bind _output_get_4 (Variables|Default|SetButton2 _returnvalue_4))
  (Variables|/Game/Blueprints/BP_Button.BP_Button_C|Setconsole _output_get_4 self)
  (bind _returnvalue_5 (Game|SpawnActorfromClass "/Game/Blueprints/BP_Button.BP_Button_C" (Math|Transform|MakeTransform (Transformation|GetWorldLocation (Variables|Default|GetVentButton3)) "0, 0, 0" "0.200000,0.200000,0.200000") "Undefined" 0 "" 0 0))
  (bind _output_get_5 (Variables|Default|SetButton3 _returnvalue_5))
  (Variables|/Game/Blueprints/BP_Button.BP_Button_C|Setconsole _output_get_5 self)
  (bind _returnvalue_6 (Game|SpawnActorfromClass "/Game/Blueprints/BP_Button.BP_Button_C" (Math|Transform|MakeTransform (Transformation|GetWorldLocation (Variables|Default|GetVentButton4)) "0, 0, 0" "0.200000,0.200000,0.200000") "Undefined" 0 "" 0 0))
  (bind _output_get_6 (Variables|Default|SetButton4 _returnvalue_6))
  (Variables|/Game/Blueprints/BP_Button.BP_Button_C|Setconsole _output_get_6 self)
  (Variables|Default|SetscaleIndicatorXMax (.x (Transformation|GetWorldScale (Variables|Default|GetV1_Pressure_indicator))))
  (Variables|Default|SetlocationIndicatorZMax (.z (Transformation|GetWorldLocation (Variables|Default|GetV1_Pressure_indicator))))
  (Variables|Default|SetcoreTemperature (Math|Random|RandomFloatinRange 5e+01 8e+01))
  (Variables|/Game/Blueprints/BP_Button.BP_Button_C|SetbuttonName (Variables|Default|GetButton1) "V1")
  (Variables|/Game/Blueprints/BP_Button.BP_Button_C|SetbuttonName (Variables|Default|GetButton2) "V2")
  (Variables|/Game/Blueprints/BP_Button.BP_Button_C|SetbuttonName (Variables|Default|GetButton3) "V3")
  (Variables|/Game/Blueprints/BP_Button.BP_Button_C|SetbuttonName (Variables|Default|GetButton4) "V4")
  (Audio|Components|Audio|SetSound (Variables|Default|GettempWarningSound) (Variables|Default|GetSW_tempWarning))
  (Audio|Components|Audio|SetSound (Variables|Default|GettempPressureSound) (Variables|Default|GetSW_pressWarning))
  (Variables|Default|SetV1Pressure (Math|Random|RandomFloatinRange 6e+01 8e+01))
  (Variables|Default|SetV2Pressure (Math|Random|RandomFloatinRange 6e+01 8e+01))
  (Variables|Default|SetV3Pressure (Math|Random|RandomFloatinRange 6e+01 8e+01))
  (Variables|Default|SetV4Pressure (Math|Random|RandomFloatinRange 6e+01 8e+01)))

(event EventTick
  (params (DeltaSeconds :type Float%20%28single-precision%29))
  (if (Variables|/Game/Blueprints/BP_Player.BP_Player_C|GetisPlaying (Variables|Default|Getplayer))
    (CallFunction|PerFrameChecks)
    (CallFunction|WarningManager)))

(fn ConstructionScript)

(fn CalculateIndicators
  (params (target :type Static%20Mesh%20Component%20Object%20Reference) (pressure :type Float%20%28single-precision%29))
  (bind _returnvalue (Transformation|GetWorldScale target))
  (bind _relativelocation (Variables|/Script/Engine.SceneComponent|GetRelativeLocation target))
  (Transformation|SetWorldScale3D target (Math|Vector|MakeVector (/ (* pressure (Variables|Default|GetscaleIndicatorXMax)) 1e+02) (.y _returnvalue) (.z _returnvalue)))
  (Transformation|SetRelativeLocation target (Math|Vector|MakeVector (.x _relativelocation) (.y _relativelocation) (Math|Float|Lerp 162.0 142.0 (- 1.0 (/ pressure 1e+02)))) false false))

(fn CalculateTemp
  (bind _deltapressure (Variables|Default|GetdeltaPressure))
  (return (+ (+ (* (Variables|Default|GetV1Pressure) _deltapressure) (* (Variables|Default|GetV2Pressure) _deltapressure) (* _deltapressure (Variables|Default|GetV3Pressure)) (* _deltapressure (Variables|Default|GetV4Pressure)) (* (Variables|Default|Getfires) (Variables|Default|GetdeltaFires))) (Variables|Default|GetcoreTemperature) (* (Variables|Default|GetdeltaRefrigeration) (Math|Float|Lerp 0.5 -0.6 (/ (Variables|Default|GetrefrigerationUnits) (Variables|Default|GetrefrigerationEfectivity)))) 0.0)))

(fn CalcualtePressure
  (params (pressure :type Float%20%28single-precision%29))
  (return (+ pressure (/ (Variables|Default|GetcoreTemperature) 1.5e+04))))

(fn ManageButtons
  (params (valve :type String))
  (bind _refrigerationunits (Variables|Default|GetrefrigerationUnits))
  (bind _usedunits (Variables|Default|GetUsedUnits))
  (bind _v2dead (Variables|Default|Getv2Dead))
  (bind _v1dead (Variables|Default|Getv1Dead))
  (bind _v3dead (Variables|Default|Getv3Dead))
  (bind _gamecontrol (Variables|Default|GetGameControl))
  (bind _returnvalue (not _v1dead))
  (bind _returnvalue_2 (not _v3dead))
  (bind _returnvalue_3 (not _v2dead))
  (bind _refrigerationunitsavailable (Variables|/Game/Blueprints/BP_GameControl.BP_GameControl_C|GetrefrigerationUnitsAvailable _gamecontrol))
  (switch string valve
    (:V1
      (if (and _returnvalue (> (- (Variables|Default|GetV1Pressure) (Variables|Default|GetpressureSubstractor)) 0.0))
        (Variables|Default|SetV1Pressure (- (Variables|Default|GetV1Pressure) (Variables|Default|GetpressureSubstractor)))
        (elif _returnvalue
          (Variables|Default|SetV1Pressure 0.0))))
    (:V2
      (if (and _returnvalue_3 (> (- (Variables|Default|GetV2Pressure) (Variables|Default|GetpressureSubstractor)) 0.0))
        (Variables|Default|SetV2Pressure (- (Variables|Default|GetV2Pressure) (Variables|Default|GetpressureSubstractor)))
        (elif _returnvalue_3
          (Variables|Default|SetV2Pressure 0.0))))
    (:V3
      (if (and _returnvalue_2 (> (- (Variables|Default|GetV3Pressure) (Variables|Default|GetpressureSubstractor)) 0.0))
        (bind _output_get (Variables|Default|SetV3Pressure (- (Variables|Default|GetV3Pressure) (Variables|Default|GetpressureSubstractor))))
        (elif _returnvalue_2
          (Variables|Default|SetV3Pressure 0.0)))
      (Development|PrintString (Utilities|String|ToString(Float) _output_get)))
    (:V4
      (if (and (not (Variables|Default|Getv4Dead)) (> (- (Variables|Default|GetV4Pressure) (Variables|Default|GetpressureSubstractor)) 0.0))
        (Variables|Default|SetV4Pressure (- (Variables|Default|GetV4Pressure) (Variables|Default|GetpressureSubstractor)))))
    (:AddButton
      (if (and (< (Variables|Default|GetrefrigerationUnits) 2e+01) (> _refrigerationunitsavailable 0.0))
        (Math|Float|IncrementFloat (Variables|Default|GetrefrigerationUnits)
          (:%20%20
            (Math|Float|DecrementFloat _refrigerationunitsavailable
              (:%20%20
                _)))))
      (if (< _refrigerationunits 1e+01) :!label _label
        (Rendering|Components|TextRender|SetText _usedunits (Utilities|Text|ToText(String) (Utilities|String|Append "0" (Utilities|String|ToString(Integer) (Math|Float|Truncate _refrigerationunits)))))
        (else
          (Rendering|Components|TextRender|SetText _usedunits (Utilities|Text|ToText(Float) _refrigerationunits "HalfToEven")))))
    (:SubsButton
      (if (> (Variables|Default|GetrefrigerationUnits) 0.0)
        (Math|Float|DecrementFloat (Variables|Default|GetrefrigerationUnits)
          (:%20%20
            (Math|Float|IncrementFloat _refrigerationunitsavailable
              (:%20%20
                (goto _label)))))
        (else
          (goto _label))))))

(fn PerFrameChecks
  (bind _v1_pressure_indicator (Variables|Default|GetV1_Pressure_indicator))
  (bind _availableunits (Variables|Default|GetAvailableUnits))
  (bind _v2_pressure_indicator (Variables|Default|GetV2_Pressure_indicator))
  (bind _gamecontrol (Variables|Default|GetGameControl))
  (bind _v3_pressure_indicator (Variables|Default|GetV3_Pressure_indicator))
  (bind _v4_pressure_indicator (Variables|Default|GetV4_Pressure_indicator))
  (bind _refrigerationunitsavailable (Variables|/Game/Blueprints/BP_GameControl.BP_GameControl_C|GetrefrigerationUnitsAvailable _gamecontrol))
  (if (< _refrigerationunitsavailable 1e+01)
    (Rendering|Components|TextRender|SetText _availableunits (Utilities|Text|ToText(String) (Utilities|String|Append "0" (Utilities|String|ToString(Integer) (Math|Float|Truncate _refrigerationunitsavailable)))))
    (else
      (Rendering|Components|TextRender|SetText _availableunits (Utilities|Text|ToText(Float) _refrigerationunitsavailable "HalfToEven"))))
  (CallFunction|CalculateIndicators (Variables|Default|GetV1_Pressure_indicator) (Variables|Default|GetV1Pressure))
  (CallFunction|CalculateIndicators (Variables|Default|GetV2_Pressure_indicator) (Variables|Default|GetV2Pressure))
  (CallFunction|CalculateIndicators (Variables|Default|GetV3_Pressure_indicator) (Variables|Default|GetV3Pressure))
  (CallFunction|CalculateIndicators (Variables|Default|GetV4_Pressure_indicator) (Variables|Default|GetV4Pressure))
  (Rendering|Components|TextRender|SetText (Variables|Default|GetTemperature) (Utilities|Text|ToText(String) (Utilities|String|Append (Utilities|String|ToString(Integer) (Math|Float|Truncate (Variables|Default|GetcoreTemperature))) "º")))
  (bind _return (CallFunction|CalculateTemp))
  (bind _output_get (Variables|Default|SetcoreTemperature _return))
  (if (< _output_get 2e+01)
    (Variables|Default|SetcoreTemperature 2e+01))
  (bind _return_2 (CallFunction|CalcualtePressure (Variables|Default|GetV1Pressure)))
  (bind _output_get_2 (Variables|Default|SetV1Pressure _return_2))
  (if (> _output_get_2 1e+02)
    (bind _returnvalue (Rendering|Material|CreateDynamicMaterialInstance _v1_pressure_indicator 0 "/Game/Materials/MT_Emergency.MT_Emergency" "None" :!class /Script/Engine.PrimitiveComponent))
    (Rendering|Material|SetMaterial _v1_pressure_indicator 0 _returnvalue)
    (Variables|Default|SetV1Pressure 1e+02)
    (Variables|Default|Setv1Dead true))
  (bind _return_3 (CallFunction|CalcualtePressure (Variables|Default|GetV2Pressure)))
  (bind _output_get_3 (Variables|Default|SetV2Pressure _return_3))
  (if (> _output_get_3 1e+02)
    (bind _returnvalue_2 (Rendering|Material|CreateDynamicMaterialInstance _v2_pressure_indicator 0 "/Game/Materials/MT_Emergency.MT_Emergency" "None" :!class /Script/Engine.PrimitiveComponent))
    (Rendering|Material|SetMaterial _v2_pressure_indicator 0 _returnvalue_2)
    (Variables|Default|SetV2Pressure 1e+02)
    (Variables|Default|Setv2Dead true))
  (bind _return_4 (CallFunction|CalcualtePressure (Variables|Default|GetV3Pressure)))
  (bind _output_get_4 (Variables|Default|SetV3Pressure _return_4))
  (if (> _output_get_4 1e+02)
    (bind _returnvalue_3 (Rendering|Material|CreateDynamicMaterialInstance _v3_pressure_indicator 0 "/Game/Materials/MT_Emergency.MT_Emergency" "None" :!class /Script/Engine.PrimitiveComponent))
    (Rendering|Material|SetMaterial _v3_pressure_indicator 0 _returnvalue_3)
    (Variables|Default|SetV3Pressure 1e+02)
    (Variables|Default|Setv3Dead true))
  (bind _return_5 (CallFunction|CalcualtePressure (Variables|Default|GetV4Pressure)))
  (bind _output_get_5 (Variables|Default|SetV4Pressure _return_5))
  (if (> _output_get_5 1e+02)
    (bind _returnvalue_4 (Rendering|Material|CreateDynamicMaterialInstance _v4_pressure_indicator 0 "/Game/Materials/MT_Emergency.MT_Emergency" "None" :!class /Script/Engine.PrimitiveComponent))
    (Rendering|Material|SetMaterial _v4_pressure_indicator 0 _returnvalue_4)
    (Variables|Default|SetV4Pressure 1e+02)
    (Variables|Default|Setv4Dead true)))

(fn WarningManager
  (bind _v1pressure (Variables|Default|GetV1Pressure))
  (bind _v2pressure (Variables|Default|GetV2Pressure))
  (bind _v4pressure (Variables|Default|GetV4Pressure))
  (bind _v3pressure (Variables|Default|GetV3Pressure))
  (bind _returnvalue (> _v3pressure 8e+01))
  (bind _returnvalue_2 (> _v1pressure 8e+01))
  (bind _returnvalue_3 (> _v4pressure 8e+01))
  (bind _returnvalue_4 (> _v2pressure 8e+01))
  (bind _returnvalue_5 (Math|Boolean|ORBoolean _returnvalue_2 _returnvalue_4 _returnvalue _returnvalue_3))
  (if (and (> (Variables|Default|GetcoreTemperature) 1.5e+02) (not (Variables|Default|GettempWarning)))
    (Utilities|Array|Add (Variables|/Game/Blueprints/BP_GameControl.BP_GameControl_C|GetwarningQueue (Variables|Default|GetGameControl)) (Variables|Default|GettempWarningSound))
    (Variables|Default|SettempWarning true)
    (elif (and (< (Variables|Default|GetcoreTemperature) 1.5e+02) (Variables|Default|GettempWarning))
      (Variables|Default|SettempWarning false)))
  (if (and _returnvalue_5 (not (Variables|Default|GetpressureWarning)))
    (Utilities|Array|Add (Variables|/Game/Blueprints/BP_GameControl.BP_GameControl_C|GetwarningQueue (Variables|Default|GetGameControl)) (Variables|Default|GettempPressureSound))
    (Variables|Default|SetpressureWarning true)
    (elif (and (Variables|Default|GetpressureWarning) (not _returnvalue_5))
      (Variables|Default|SetpressureWarning false))))