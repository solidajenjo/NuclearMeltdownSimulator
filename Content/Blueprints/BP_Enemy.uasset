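; BP_Enemy is an enemy that homes in on the player with a pulsing six-part body, playing a noise on spawn.
; While the player is playing, Tick turns it to face the player on the horizontal plane, raises it until it passes a set height, and moves it forward.
; Six randomized timers update each mesh's scale direction, and RescaleParts scales them within limits.
; It destroys itself when the player is dead.
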(event EventBeginPlay
  (Variables|Default|Settimer (Math|Random|RandomFloatinRange 0.5 1.5))
  (Variables|Default|Settimer_0 (Math|Random|RandomFloatinRange 0.5 1.5))
  (Variables|Default|Settimer_1 (Math|Random|RandomFloatinRange 0.5 1.5))
  (Variables|Default|Settimer_2 (Math|Random|RandomFloatinRange 0.5 1.5))
  (Variables|Default|Settimer_3 (Math|Random|RandomFloatinRange 0.5 1.5))
  (Variables|Default|Settimer_4 (Math|Random|RandomFloatinRange 0.5 1.5))
  (bind _asbp_player (Utilities|Casting|CastToBP_Player (Game|Player|GetPlayerPawn 0)))
  (bind _output_get (Variables|Default|Setplayer _asbp_player))
  (if (Variables|/Game/Blueprints/BP_Player.BP_Player_C|GetisDead _output_get)
    (Actor|DestroyActor)
    (else
      (Audio|Components|Audio|Play (Variables|Default|Getnoise) 0.0))))

(event Collision|EventActorBeginOverlap
  (params (OtherActor :type Actor%20Object%20Reference)))

(event EventTick
  (params (DeltaSeconds :type Float%20%28single-precision%29))
  (bind _player (Variables|Default|Getplayer))
  (bind _defaultsceneroot (Variables|Default|GetDefaultSceneRoot))
  (bind _player_2 (Variables|Default|Getplayer))
  (bind _returnvalue (Transformation|GetWorldLocation _defaultsceneroot))
  (bind _rootcomponent (Variables|/Script/Engine.Actor|GetRootComponent _player_2))
  (bind _returnvalue_2 (Transformation|GetWorldLocation _rootcomponent))
  (if (Variables|/Game/Blueprints/BP_Player.BP_Player_C|GetisDead (Variables|Default|Getplayer))
    (Actor|DestroyActor))
  (if (Variables|/Game/Blueprints/BP_Player.BP_Player_C|GetisPlaying _player)
    (if (not (Variables|/Game/Blueprints/BP_Player.BP_Player_C|GetisDead _player))
      (Utilities|Timers DeltaSeconds DeltaSeconds
        (:next
          (Transformation|SetActorRotation (Math|Rotator|FindLookatRotation (Math|Vector|MakeVector (.x _returnvalue) (.y _returnvalue) (.z _returnvalue)) (Math|Vector|MakeVector (.x _returnvalue_2) (.y _returnvalue_2) (.z _returnvalue))))
          (Utilities|Reescalation
            (:next
              (if (and (<= (.z (Transformation|GetWorldLocation (Variables|Default|GetDefaultSceneRoot))) (Variables|Default|Getheight)) (not (Variables|Default|Gettraveling)))
                (Transformation|AddActorWorldOffset (Math|Vector|MakeVector 0.0 0.0 (* (Utilities|Time|GetWorldDeltaSeconds) (Variables|Default|Getspeed))))
                (else
                  (Variables|Default|Settraveling true)))
              (Transformation|AddActorWorldOffset (* (Math|Vector|GetForwardVector (Variables|Default|GetDefaultSceneRoot)) (* (Variables|Default|Getspeed) (Utilities|Time|GetWorldDeltaSeconds)))))))))))

(fn ConstructionScript)

(fn RescaleParts
  (params (self2 :type Scene%20Component%20Object%20Reference) (self3 :type Scene%20Component%20Object%20Reference) (scaleDir :type Float%20%28single-precision%29))
  (bind _returnvalue (Utilities|Time|GetWorldDeltaSeconds))
  (bind _minscale (Variables|Default|GetminScale))
  (bind _maxscale (Variables|Default|GetmaxScale))
  (bind _relativescale3d (Variables|/Script/Engine.SceneComponent|GetRelativeScale3D self3))
  (bind _scalespeed (Variables|Default|GetscaleSpeed))
  (bind _returnvalue_2 (* _scalespeed _returnvalue scaleDir))
  (bind _returnvalue_3 (+ _relativescale3d _returnvalue_2))
  (if (Math|Boolean|ANDBoolean (> (.x _returnvalue_3) _minscale) (> (.y _returnvalue_3) _minscale) (> (.z _returnvalue_3) _minscale) (< (.x _returnvalue_3) _maxscale) (< (.y _returnvalue_3) _maxscale) (< (.z _returnvalue_3) _maxscale))
    (Transformation|SetRelativeScale3D self2 (Math|Vector|MakeVector (.x _returnvalue_3) (.y _returnvalue_3) (.z _returnvalue_3)))))