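; BP_GameControl is a game control actor that links itself to four BP_Console child actors.
; On BeginPlay it casts each console's child actor in turn and sets that console's GameControl reference to itself.
; The casts are chained, so one failure leaves the remaining consoles unlinked.
; Tick and the construction script are empty.
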(event EventBeginPlay
  (bind _asbp_console (Utilities|Casting|CastToBP_Console (Variables|/Script/Engine.ChildActorComponent|GetChildActor (Variables|Default|GetConsole1))))
  (Variables|/Game/Blueprints/BP_Console.BP_Console_C|SetGameControl _asbp_console self)
  (bind _asbp_console_2 (Utilities|Casting|CastToBP_Console (Variables|/Script/Engine.ChildActorComponent|GetChildActor (Variables|Default|GetConsole2))))
  (Variables|/Game/Blueprints/BP_Console.BP_Console_C|SetGameControl _asbp_console_2 self)
  (bind _asbp_console_3 (Utilities|Casting|CastToBP_Console (Variables|/Script/Engine.ChildActorComponent|GetChildActor (Variables|Default|GetConsole3))))
  (Variables|/Game/Blueprints/BP_Console.BP_Console_C|SetGameControl _asbp_console_3 self)
  (bind _asbp_console_4 (Utilities|Casting|CastToBP_Console (Variables|/Script/Engine.ChildActorComponent|GetChildActor (Variables|Default|GetConsole4))))
  (Variables|/Game/Blueprints/BP_Console.BP_Console_C|SetGameControl _asbp_console_4 self))

(event EventTick
  (params (DeltaSeconds :type Float%20%28single-precision%29)))

(fn ConstructionScript)