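; Cone actor that acts as a leaking enemy spawner, creating scaled-down BP_Enemy actors at its SplashLoc point.
; Tick runs a countdown, printed on screen for debugging, and on expiry spawns an enemy and picks a new random delay.
; The delay range shrinks after each spawn until its minimum reaches a floor, so spawns grow more frequent.
; Collisions from the PT_Leak particles trigger a nuclear splash emitter at the same point.
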(event OnParticleCollide(PT_Leak)
  (params (EventName :type Name :default "None") (EmitterTime :type Float%20%28single-precision%29) (ParticleTime :type Integer) (Location :type Vector :default "0, 0, 0") (Velocity :type Vector :default "0, 0, 0") (Direction :type Vector :default "0, 0, 0") (Normal :type Vector :default "0, 0, 0") (BoneName :type Name :default "None") (PhysMat :type Physical%20Material%20Object%20Reference))
  (Effects|SpawnEmitteratLocation "/Game/Particles/PT_Nuclear_splash.PT_Nuclear_splash" (Transformation|GetWorldLocation (Variables|Default|GetsplashLoc))))

(event EventBeginPlay)

(event Collision|EventActorBeginOverlap
  (params (OtherActor :type Actor%20Object%20Reference)))

(event EventTick
  (params (DeltaSeconds :type Float%20%28single-precision%29))
  (Development|PrintString (Utilities|String|ToString(Float) (Variables|Default|Gettimer)))
  (if (<= (Variables|Default|Gettimer) 0.0)
    (Game|SpawnActorfromClass "/Game/Blueprints/BP_Enemy.BP_Enemy_C" (Math|Transform|MakeTransform (Transformation|GetWorldLocation (Variables|Default|GetsplashLoc)) "0, 0, 0" "0.200000,0.200000,0.200000") "Undefined" 0 0)
    (Variables|Default|Settimer (Math|Random|RandomFloatinRange (Variables|Default|GetminTime) (Variables|Default|GetmaxTime)))
    (if (> (Variables|Default|GetminTime) 15.0)
      (Math|Float|DecrementFloat (Variables|Default|GetminTime)
        (:%20%20
          (Math|Float|DecrementFloat (Variables|Default|GetmaxTime)))))
    (else
      (Variables|Default|Settimer (- (Variables|Default|Gettimer) (Utilities|Time|GetWorldDeltaSeconds))))))

(fn ConstructionScript)