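; BP_Console2 is the sprinkler console where the player puts out random fires across four reactors.
; On BeginPlay it registers with GameControl and spawns 32 button and red/green light units, eight per reactor.
; While the player is playing, Tick randomly ignites units, clears pressed ones, updates lights and counts fires per reactor.
; The fireAlarms macro queues timer-throttled reactor warnings in GameControl, while fire probability ramps up to a cap.
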(event EventBeginPlay
  (bind _asbp_player (Utilities|Casting|CastToBP_Player (Game|Player|GetPlayerPawn 0)))
  (Variables|Default|Setplayer _asbp_player)
  (Variables|/Game/Blueprints/BP_GameControl.BP_GameControl_C|Setconsole2 (Variables|Default|GetgameControl) self)
  (Utilities|InitConsole))

(event Collision|EventActorBeginOverlap
  (params (OtherActor :type Actor%20Object%20Reference)))

(event EventTick
  (params (DeltaSeconds :type Float%20%28single-precision%29))
  (if (Variables|/Game/Blueprints/BP_Player.BP_Player_C|GetisPlaying (Variables|Default|Getplayer))
    (Variables|Default|SetbWarningTimerR1_0 false)
    (Variables|Default|SetbWarningTimerR2_0 false)
    (Variables|Default|SetbWarningTimerR3_0 false)
    (Variables|Default|SetbWarningTimerR4_0 false)
    (Variables|Default|Setr1Fires 0.0)
    (Variables|Default|Setr2Fires 0.0)
    (Variables|Default|Setr3Fires 0.0)
    (Variables|Default|Setr4Fires 0.0)
    (for (_array_element _array_index) (Variables|Default|GetcontrolPanel)
      (Utilities|ControlPanelLogic _array_element _array_index _array_index DeltaSeconds))
    (if (< (+ (Variables|Default|GetfireProbability) (* (Variables|Default|GetdeltaFireProbability) DeltaSeconds)) 0.01)
      (Variables|Default|SetfireProbability (+ (Variables|Default|GetfireProbability) (* (Variables|Default|GetdeltaFireProbability) DeltaSeconds))))))

(fn ConstructionScript)

(fn PutComponents
  (params (self2 :type Scene%20Component%20Object%20Reference) (reactor :type String))
  (bind _returnvalue (Transformation|GetWorldLocation self2))
  (bind _returnvalue_2 (- (.y _returnvalue) 1.0))
  (bind _returnvalue_3 (Game|SpawnActorfromClass "/Game/Blueprints/BP_sprinklerControl.BP_sprinklerControl_C" (Math|Transform|MakeTransform (Math|Vector|MakeVector (.x _returnvalue) _returnvalue_2 (.z _returnvalue)) "0, 0, 0" "0.150000,0.150000,0.150000") "Undefined" 0 0))
  (bind _returnvalue_4 (Game|SpawnActorfromClass "/Game/Blueprints/BP_Button.BP_Button_C" (Math|Transform|MakeTransform (Math|Vector|MakeVector (- (.x _returnvalue) 6.5) (- _returnvalue_2 1e+01) (- (.z _returnvalue) 21.5)) "0, 0,180.000000" "0.150000,0.150000,0.150000") "Undefined" 0 "Console2 button" 3 0))
  (bind _output_get (LocalVariables|SetnewSprinklerUnit (Utilities|Struct|MakeBP_SprinklerUnit _returnvalue_4 (Variables|/Game/Blueprints/BP_sprinklerControl.BP_sprinklerControl_C|GetChildActor _returnvalue_3) (Variables|/Game/Blueprints/BP_sprinklerControl.BP_sprinklerControl_C|GetChildActor1 _returnvalue_3) false reactor)))
  (Utilities|Array|Add (Variables|Default|GetcontrolPanel) _output_get)
  (return))